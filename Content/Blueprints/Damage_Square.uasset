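; Damage_Square is a damageable hazard actor that hurts the player on contact and can be destroyed by weapons.
; Collision overlap deals fixed damage to a SkilledCharacter, briefly clearing its PlayerHitable flag.
; Art, Design or Dev weapon overlaps apply that weapon's Damage, play a sound and start a timed IsHittable cooldown.
; Tick destroys the actor once Health reaches zero or below.
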(event OnComponentBeginOverlap(Collision)
  (params (OverlappedComponent :type Primitive%20Component%20Object%20Reference) (OtherActor :type Actor%20Object%20Reference) (OtherComp :type Primitive%20Component%20Object%20Reference) (OtherBodyIndex :type Integer) (bFromSweep :type Boolean) (SweepResult :type Hit%20Result%20Structure%20%28by%20ref%29))
  (bind _asskilled_character (Utilities|Casting|CastToSkilledCharacter OtherActor)
    (:then
      (if (Variables|/Game/Blueprints/SkilledCharacter.SkilledCharacter_C|GetplayerHitable _asskilled_character)
        (Default|DamagePlayer _asskilled_character 1e+01)
        (Variables|/Game/Blueprints/SkilledCharacter.SkilledCharacter_C|SetplayerHitable _asskilled_character false)
        (Utilities|FlowControl|Delay 0.2)
        (Variables|/Game/Blueprints/SkilledCharacter.SkilledCharacter_C|SetplayerHitable _asskilled_character true)))
    (:CastFailed
      (bind _asweapon_art (Utilities|Casting|CastToWeapon_Art OtherActor)
        (:then
          (if (Variables|Default|GetisHittable)
            (CallFunction|EnemyDamaged (Variables|/Game/Blueprints/Weapon_Art.Weapon_Art_C|GetDamage _asweapon_art))
            (Variables|Default|SetisHittable false :!label _label)
            (Audio|PlaySound2D 0 1.0 1.0 0.0 0 0)
            (Utilities|FlowControl|Delay 2.0)
            (Variables|Default|SetisHittable true)))
        (:CastFailed
          (bind _asweapon_gdd (Utilities|Casting|CastToWeapon_Design OtherActor)
            (:then
              (if (Variables|Default|GetisHittable)
                (CallFunction|EnemyDamaged (Variables|/Game/Blueprints/Weapon_Design.Weapon_Design_C|GetDamage _asweapon_gdd))
                (goto _label)))
            (:CastFailed
              (bind _asweapon_kb (Utilities|Casting|CastToWeapon_Dev OtherActor))
              (if (Variables|Default|GetisHittable)
                (CallFunction|EnemyDamaged (Variables|/Game/Blueprints/Weapon_Dev.Weapon_Dev_C|GetDamage _asweapon_kb))
                (goto _label)))))))))

(event Custom|Enemy_Damaged
  (params (Damage :type Float%20%28single-precision%29))
  (Variables|Default|SetHealth (- (Variables|Default|GetHealth) Damage)))

(event EventBeginPlay)

(event EventTick
  (params (DeltaSeconds :type Float%20%28single-precision%29))
  (Utilities|FlowControl|Sequence
    (:then_0
      (if (<= (Variables|Default|GetHealth) 0.0)
        (Actor|DestroyActor)))))

(fn ConstructionScript)