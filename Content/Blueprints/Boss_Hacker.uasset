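; Hacker boss enemy that swings a weapon, summons Enemy_Runner waves, and finishes the level when its health runs out.
; Sighting the player triggers three escalating one-time waves gated by health, spawned through a delayed-loop macro.
; Tick repeats the timer-driven swing after each cooldown and toggles IsHittable and the mesh by whether tagged minions remain.
; Player weapon overlaps subtract health without checking IsHittable; box overlaps damage hittable players mid-swing.
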(event OnSeePawn(PawnSensing)
  (params (Pawn :type Pawn%20Object%20Reference))
  (Utilities|Casting|CastToSkilledCharacter Pawn)
  (if (Variables|Default|GetfirstSpawnCompleted)
    (if (<= (Variables|Default|GetBasic_Health) 3.5e+02)
      (if (Variables|Default|GetsecondSpawnCompleted)
        (if (<= (Variables|Default|GetBasic_Health) 1.5e+02)
          (if (not (Variables|Default|GetthirdSpawnCompleted))
            (Variables|Default|SetthirdSpawnCompleted true)
            (CallFunction|SpawnMinions 7 2.0)))
        (else
          (Variables|Default|SetsecondSpawnCompleted true)
          (CallFunction|SpawnMinions 6 2.0))))
    (else
      (Variables|Default|SetfirstSpawnCompleted true)
      (CallFunction|SpawnMinions 5 2.0))))

(event OnComponentBeginOverlap(CapsuleComponent)
  (params (OverlappedComponent :type Primitive%20Component%20Object%20Reference) (OtherActor :type Actor%20Object%20Reference) (OtherComp :type Primitive%20Component%20Object%20Reference) (OtherBodyIndex :type Integer) (bFromSweep :type Boolean) (SweepResult :type Hit%20Result%20Structure%20%28by%20ref%29))
  (bind _asweapon_art (Utilities|Casting|CastToWeapon_Art OtherActor)
    (:then
      (CallFunction|BasicDamaged (Variables|/Game/Blueprints/Weapon_Art.Weapon_Art_C|GetDamage _asweapon_art)))
    (:CastFailed
      (bind _asweapon_design (Utilities|Casting|CastToWeapon_Design OtherActor)
        (:then
          (CallFunction|BasicDamaged (Variables|/Game/Blueprints/Weapon_Design.Weapon_Design_C|GetDamage _asweapon_design)))
        (:CastFailed
          (bind _asweapon_dev (Utilities|Casting|CastToWeapon_Dev OtherActor)
            (:then
              (CallFunction|BasicDamaged (Variables|/Game/Blueprints/Weapon_Dev.Weapon_Dev_C|GetDamage _asweapon_dev)))
            (:CastFailed
              (bind _asweapon_art_supper (Utilities|Casting|CastToWeapon_ArtSupper OtherActor)
                (:then
                  (CallFunction|BasicDamaged (Variables|/Game/Blueprints/Weapon_ArtSupper.Weapon_ArtSupper_C|GetDamage _asweapon_art_supper)))
                (:CastFailed
                  (bind _asweapon_design_supper (Utilities|Casting|CastToWeapon_DesignSupper OtherActor)
                    (:then
                      (CallFunction|BasicDamaged (Variables|/Game/Blueprints/Weapon_DesignSupper.Weapon_DesignSupper_C|GetDamage _asweapon_design_supper)))
                    (:CastFailed
                      (bind _asweapon_dev_super (Utilities|Casting|CastToWeapon_DevSuper OtherActor))
                      (CallFunction|BasicDamaged (Variables|/Game/Blueprints/Weapon_DevSuper.Weapon_DevSuper_C|GetDamage _asweapon_dev_super))))))))))))
  (Audio|PlaySound2D 0 1.0 1.0 0.0 0 0))

(event OnComponentBeginOverlap(Box)
  (params (OverlappedComponent :type Primitive%20Component%20Object%20Reference) (OtherActor :type Actor%20Object%20Reference) (OtherComp :type Primitive%20Component%20Object%20Reference) (OtherBodyIndex :type Integer) (bFromSweep :type Boolean) (SweepResult :type Hit%20Result%20Structure%20%28by%20ref%29))
  (bind _asskilled_character (Utilities|Casting|CastToSkilledCharacter OtherActor))
  (if (Variables|/Game/Blueprints/SkilledCharacter.SkilledCharacter_C|GetplayerHitable _asskilled_character)
    (if (Variables|Default|GetweaponUp)
      (Default|DamagePlayer _asskilled_character 2e+01))))

(event Custom|BasicDamaged
  (params (Damage :type Float%20%28single-precision%29))
  (Variables|Default|SetBasic_Health (- (Variables|Default|GetBasic_Health) Damage)))

(event Custom|Attack_SwingLeft
  ;[1 1 1] Attack
  (Transformation|AddLocalRotation (Variables|Default|GetWeapon) "0,-8.000000, 0" false false))

(event Custom|Attack_SwingRight
  ;[1 1 1] Attack
  (Transformation|AddLocalRotation (Variables|Default|GetWeapon) "0,8.000000, 0" false false))

(event Custom|SpawnMinions
  (params (Amount :type Integer) (Cooldown :type Float%20%28single-precision%29))
  (Utilities|ForLoopwithDelay 1 Amount Cooldown
    (:Loop%20Body
      (bind _returnvalue (AI|SpawnAIFromClass "/Game/Blueprints/Enemy_Runner.Enemy_Runner_C" 0 (Transformation|GetWorldLocation (Variables|Default|GetEnemySpawn)) "0, 0, 0" false 0))
      (Utilities|FlowControl|Delay 0.2)
      (Variables|/Script/Engine.Actor|SetTags _returnvalue (Utilities|Array|MakeArray "Boss")))))

(event Custom|Attack
  ;[1 1 1] Attack
  (Variables|Default|SetcanUseWeapon false)
  (Variables|Default|SetweaponUp true)
  (bind _returnvalue (Utilities|Time|SetTimerbyFunctionName 0 "Attack_SwingLeft" 0.02 true))
  (Utilities|FlowControl|Delay 0.5)
  (Utilities|Time|ClearandInvalidateTimerbyHandle _returnvalue)
  (bind _returnvalue_2 (Utilities|Time|SetTimerbyFunctionName 0 "Attack_SwingRight" 0.02 true))
  (Utilities|FlowControl|Delay 0.5)
  (Utilities|Time|ClearandInvalidateTimerbyHandle _returnvalue_2)
  (Variables|Default|SetweaponUp false)
  (Utilities|FlowControl|Delay 3.0)
  (Variables|Default|SetcanUseWeapon true))

(event EventTick
  (params (DeltaSeconds :type Float%20%28single-precision%29))
  (bind _staticmesh (Variables|Default|GetStaticMesh))
  (Utilities|FlowControl|Sequence
    (:then_0
      (if (<= (Variables|Default|GetBasic_Health) 0.0)
        (bind _asdcu_game_mode (Utilities|Casting|CastToDCU_GameMode (Game|GetGameMode)))
        (Default|FinishedLevel _asdcu_game_mode)
        (Actor|DestroyActor)))
    (:then_1
      (bind _outactors (Actor|GetAllActorsOfClasswithTag "/Game/Blueprints/Enemy_Runner.Enemy_Runner_C" "Boss"))
      (if (<= (Utilities|Array|Length _outactors) 0)
        (Variables|Default|SetisHittable true)
        (else
          (Variables|Default|SetisHittable false))))
    (:then_2
      (if (Variables|Default|GetisHittable)
        (Components|StaticMesh|SetStaticMesh _staticmesh 0)
        (else
          (Components|StaticMesh|SetStaticMesh _staticmesh "/Game/Meshes/EditorPH/1M_Cube_Chamfer.1M_Cube_Chamfer"))))
    (:then_3
      (if (Variables|Default|GetcanUseWeapon)
        (CallFunction|Attack)))))

(fn ConstructionScript)