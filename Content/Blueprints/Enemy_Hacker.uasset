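; Enemy Hacker pawn that pursues sensed pawns with ranged and melee attacks, halting if it sees one while the game state's HackIsOn is set.
; Each move order triggers cooldown-gated EnemyWeapon_KB shots; arrival triggers a timer-driven weapon swing.
; Its box overlap damages and calls WeakPlayer on the player while WeaponUp.
; Capsule overlaps with six player weapon classes reduce health with brief invulnerability, and Tick destroys it at zero.
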(event OnSeePawn(PawnSensing)
  (params (Pawn :type Pawn%20Object%20Reference))
  (bind _asdcu_game_state (Utilities|Casting|CastToDCU_GameState (Game|GetGameState)))
  (if (Variables|/Game/Behaviour/DCU_GameState.DCU_GameState_C|GetHackIsOn _asdcu_game_state)
    (Components|Movement|StopMovementImmediately (Variables|Character|GetCharacterMovement))
    (else
      (AI|AIMoveTo self "0, 0, 0" Pawn 5.0 false
        (:then
          (Utilities|FlowControl|Delay 0.2)
          (CallFunction|Shoot))
        (:OnSuccess
          (if (Variables|Default|GetcanHit)
            (Variables|Default|SetcanHit false)
            (Variables|Default|SetweaponUp true)
            (bind _returnvalue (Utilities|Time|SetTimerbyFunctionName 0 "Attack_SwingLeft" 0.02 true))
            (Utilities|FlowControl|Delay 0.5)
            (Utilities|Time|ClearandInvalidateTimerbyHandle _returnvalue)
            (bind _returnvalue_2 (Utilities|Time|SetTimerbyFunctionName 0 "Attack_SwingRight" 0.02 true))
            (Utilities|FlowControl|Delay 0.5)
            (Utilities|Time|ClearandInvalidateTimerbyHandle _returnvalue_2)
            (Utilities|FlowControl|Delay 1.0)
            (Variables|Default|SetcanHit true)))))))

(event OnComponentBeginOverlap(CapsuleComponent)
  (params (OverlappedComponent :type Primitive%20Component%20Object%20Reference) (OtherActor :type Actor%20Object%20Reference) (OtherComp :type Primitive%20Component%20Object%20Reference) (OtherBodyIndex :type Integer) (bFromSweep :type Boolean) (SweepResult :type Hit%20Result%20Structure%20%28by%20ref%29))
  (bind _asweapon_art (Utilities|Casting|CastToWeapon_Art OtherActor)
    (:then
      (if (Variables|Default|GetisHittable)
        (CallFunction|BasicDamaged (Variables|/Game/Blueprints/Weapon_Art.Weapon_Art_C|GetDamage _asweapon_art))
        (Variables|Default|SetisHittable false :!label _label)
        (Audio|PlaySound2D 0 1.0 1.0 0.0 0 0)
        (Utilities|FlowControl|Delay 0.3)
        (Variables|Default|SetisHittable true)))
    (:CastFailed
      (bind _asweapon_design (Utilities|Casting|CastToWeapon_Design OtherActor)
        (:then
          (if (Variables|Default|GetisHittable)
            (CallFunction|BasicDamaged (Variables|/Game/Blueprints/Weapon_Design.Weapon_Design_C|GetDamage _asweapon_design))
            (goto _label)))
        (:CastFailed
          (bind _asweapon_dev (Utilities|Casting|CastToWeapon_Dev OtherActor)
            (:then
              (if (Variables|Default|GetisHittable)
                (CallFunction|BasicDamaged (Variables|/Game/Blueprints/Weapon_Dev.Weapon_Dev_C|GetDamage _asweapon_dev))
                (goto _label)))
            (:CastFailed
              (bind _asweapon_art_supper (Utilities|Casting|CastToWeapon_ArtSupper OtherActor)
                (:then
                  (if (Variables|Default|GetisHittable)
                    (CallFunction|BasicDamaged (Variables|/Game/Blueprints/Weapon_ArtSupper.Weapon_ArtSupper_C|GetDamage _asweapon_art_supper))
                    (goto _label)))
                (:CastFailed
                  (bind _asweapon_design_supper (Utilities|Casting|CastToWeapon_DesignSupper OtherActor)
                    (:then
                      (if (Variables|Default|GetisHittable)
                        (CallFunction|BasicDamaged (Variables|/Game/Blueprints/Weapon_DesignSupper.Weapon_DesignSupper_C|GetDamage _asweapon_design_supper))
                        (goto _label)))
                    (:CastFailed
                      (bind _asweapon_dev_super (Utilities|Casting|CastToWeapon_DevSuper OtherActor))
                      (if (Variables|Default|GetisHittable)
                        (CallFunction|BasicDamaged (Variables|/Game/Blueprints/Weapon_DevSuper.Weapon_DevSuper_C|GetDamage _asweapon_dev_super))
                        (goto _label)))))))))))))

(event OnComponentBeginOverlap(Box)
  (params (OverlappedComponent :type Primitive%20Component%20Object%20Reference) (OtherActor :type Actor%20Object%20Reference) (OtherComp :type Primitive%20Component%20Object%20Reference) (OtherBodyIndex :type Integer) (bFromSweep :type Boolean) (SweepResult :type Hit%20Result%20Structure%20%28by%20ref%29))
  (bind _asskilled_character (Utilities|Casting|CastToSkilledCharacter OtherActor))
  (if (Variables|/Game/Blueprints/SkilledCharacter.SkilledCharacter_C|GetplayerHitable _asskilled_character)
    (if (Variables|Default|GetweaponUp)
      (Default|DamagePlayer _asskilled_character 5.0)
      (Variables|Default|SetweaponUp false)
      (bind _asdcu_game_state (Utilities|Casting|CastToDCU_GameState (Game|GetGameState)))
      (Default|WeakPlayer _asdcu_game_state 3.0))))

(event Custom|BasicDamaged
  (params (Damage :type Float%20%28single-precision%29))
  (Variables|Default|SetBasic_Health (- (Variables|Default|GetBasic_Health) Damage)))

(event Custom|Attack_SwingLeft
  ;[1 1 1] Attack
  (Transformation|AddLocalRotation (Variables|Default|GetWeapon) "0,-8.000000, 0" false false))

(event Custom|Attack_SwingRight
  ;[1 1 1] Attack
  (Transformation|AddLocalRotation (Variables|Default|GetWeapon) "0,8.000000, 0" false false))

(event Custom|Shoot
  (if (Variables|Default|GetcanShoot)
    (Variables|Default|SetcanShoot false)
    (Game|SpawnActorfromClass "/Game/Blueprints/EnemyWeapon_KB.EnemyWeapon_KB_C" (Transformation|GetWorldTransform (Variables|Default|GetScene)) "Undefined" 0 0)
    (Utilities|FlowControl|Delay (Variables|Default|GetshootDelay))
    (Variables|Default|SetcanShoot true)))

(event EventTick
  (params (DeltaSeconds :type Float%20%28single-precision%29))
  (Utilities|FlowControl|Sequence
    (:then_0
      (if (<= (Variables|Default|GetBasic_Health) 0.0)
        (Actor|DestroyActor)))))

(fn ConstructionScript)