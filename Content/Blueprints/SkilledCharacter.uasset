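; Player character with plane-locked movement, a cooldown dash along the camera boom, and a deck of six cyclable skill cards.
; Each card is single-use until Reload re-enables all, and every reload lengthens the next.
; Cards spawn short-lived child actors, raise a temporary shield, heal through a looping timer, or briefly set the HackIsOn flag on DCU_GameState.
; Damage and heal events adjust Health, which Tick caps at maximum.
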(event OnComponentBeginOverlap(ShieldCollision)
  (params (OverlappedComponent :type Primitive%20Component%20Object%20Reference) (OtherActor :type Actor%20Object%20Reference) (OtherComp :type Primitive%20Component%20Object%20Reference) (OtherBodyIndex :type Integer) (bFromSweep :type Boolean) (SweepResult :type Hit%20Result%20Structure%20%28by%20ref%29))
  (if (Variables|Default|GethasShield)
    (if (not (== OtherActor self))
      (if (Variables|Default|GetshieldDestroyOnHit)
        (Variables|Default|SethasShield false)
        (Variables|Default|SetshieldDestroyOnHit false)))))

(event Custom|Reload
  (params (Duration :type Float%20%28single-precision%29))
  ;[0.07827 0 1] Reload Cards
  (Utilities|FlowControl|Delay Duration)
  (Variables|Default|SetCard0_Disabled false)
  (Variables|Default|SetCard1_Disabled false)
  (Variables|Default|SetCard2_Disabled false)
  (Variables|Default|SetCard3_Disabled false)
  (Variables|Default|SetCard4_Disabled false)
  (Variables|Default|SetCard5_Disabled false)
  (Variables|Default|SetcanReload true))

(event Custom|DamagePlayer
  (params (Damage :type Float%20%28single-precision%29))
  ;[1 0.02997 0] Health Functions
  (Variables|Default|SetHealth (- (Variables|Default|GetHealth) Damage))
  (Utilities|FlowControl|Delay 0.6)
  (Variables|Default|SetplayerHitable true))

(event Custom|HealPlayer
  (params (Healing :type Float%20%28single-precision%29))
  ;[1 0.02997 0] Health Functions
  (Variables|Default|SetHealth (+ (Variables|Default|GetHealth) Healing)))

(event EventTick
  (params (DeltaSeconds :type Float%20%28single-precision%29))
  (Utilities|FlowControl|Sequence
    (:then_0
      ;[1 1 1] Fixing Overhealth
      (if (> (Variables|Default|GetHealth) 1e+02)
        (Variables|Default|SetHealth 1e+02)))))

(event Input|ActionEvents|InputActionNextCard
  (params (Key :type Key%20Structure :default "None"))
  ;[0.973 0.2339 1] Next/Previous Card
  (:Pressed
    (if (>= (Variables|Default|GetCurrentCard) 5)
      (Variables|Default|SetCurrentCard 0)
      (else
        (Math|Integer|IncrementInt (Variables|Default|GetCurrentCard))))))

(event Input|ActionEvents|InputActionPrevCard
  (params (Key :type Key%20Structure :default "None"))
  ;[0.973 0.2339 1] Next/Previous Card
  (:Pressed
    (if (<= (Variables|Default|GetCurrentCard) 0)
      (Variables|Default|SetCurrentCard 5)
      (else
        (Math|Integer|DecrementInt (Variables|Default|GetCurrentCard))))))

(event Input|ActionEvents|InputActionDash
  (params (Key :type Key%20Structure :default "None"))
  ;[1 0.8526 0] Dash Ability
  (:Pressed
    (if (Variables|Default|GetcanDash)
      (Character|LaunchCharacter (* (Math|Vector|GetForwardVector (Variables|MyCharacter|GetCameraBoom)) 1e+04) false false)
      (Variables|Default|SetcanDash false)
      (Utilities|FlowControl|Delay 1.0)
      (Variables|Default|SetcanDash true))))

(event Input|ActionEvents|InputActionUseCard
  (params (Key :type Key%20Structure :default "None"))
  ;[0 0.9379 1] Using Cards
  (:Pressed
    (switch int (Variables|Default|GetCurrentCard)
      (:0
        (if (Variables|Default|GetCard0_Disabled)
          (CallFunction|CardFail)
          (else
            (Variables|Default|SetCard0_Disabled true)
            (bind _returnvalue (AddComponent|AddChildActorComponent false))
            (Utilities|FlowControl|Delay 2.0)
            (Components|DestroyComponent _returnvalue))))
      (:1
        (if (Variables|Default|GetCard1_Disabled)
          (CallFunction|CardFail)
          (else
            (Variables|Default|SetCard1_Disabled true)
            (bind _returnvalue_2 (AddComponent|AddChildActorComponent false))
            (Utilities|FlowControl|Delay 2.0)
            (Components|DestroyComponent _returnvalue_2))))
      (:2
        (if (Variables|Default|GetCard2_Disabled)
          (CallFunction|CardFail)
          (else
            (Variables|Default|SetCard2_Disabled true)
            (bind _returnvalue_3 (AddComponent|AddChildActorComponent false))
            (Utilities|FlowControl|Delay 2.0)
            (Components|DestroyComponent _returnvalue_3))))
      (:3
        (if (Variables|Default|GetCard3_Disabled)
          (CallFunction|CardFail)
          (else
            (Variables|Default|SetCard3_Disabled true)
            (CallFunction|SkillGDDShield false)
            (Utilities|FlowControl|Delay 5.0)
            (Components|StaticMesh|SetStaticMesh (Variables|Default|GetShield) 0)
            (Variables|Default|SethasShield false))))
      (:4
        (if (Variables|Default|GetCard4_Disabled)
          (CallFunction|CardFail)
          (else
            (Variables|Default|SetCard4_Disabled true)
            (bind _returnvalue_4 (Utilities|Time|SetTimerbyFunctionName 0 "Skill_PaintbrushHeal" 0.2 true))
            (Utilities|FlowControl|Delay 1.0)
            (Utilities|Time|ClearandInvalidateTimerbyHandle _returnvalue_4))))
      (:5
        (if (Variables|Default|GetCard5_Disabled)
          (CallFunction|CardFail)
          (else
            (Variables|Default|SetCard5_Disabled true)
            (CallFunction|SkillProgramHack)
            (Utilities|FlowControl|Delay 2.0)
            (bind _asdcu_game_state (Utilities|Casting|CastToDCU_GameState (Game|GetGameState)))
            (Variables|/Game/Behaviour/DCU_GameState.DCU_GameState_C|SetHackIsOn _asdcu_game_state false)))))))

(event Input|ActionEvents|InputActionReload
  (params (Key :type Key%20Structure :default "None"))
  (bind _reloadtime (Variables|Default|GetReloadTime))
  (bind _returnvalue (Math|Conversions|ToFloat(Integer) _reloadtime))
  ;[0.973 0.2339 1] Next/Previous Card
  (:Pressed
    (if (Variables|Default|GetcanReload)
      (Variables|Default|SetcanReload false)
      (CallFunction|Reload _returnvalue)
      (Utilities|FlowControl|Delay _returnvalue)
      (Math|Integer|IncrementInt _reloadtime))))

(event Input|AxisEvents|InputAxisMoveForward
  (params (AxisValue :type Float%20%28single-precision%29))
  ;[0 1 0.1055] Basic Movement
  (Pawn|Input|AddMovementInput (Math|Vector|GetForwardVector (Math|Rotator|MakeRotator 0.0 0.0 (.Yaw (Math|Rotator|BreakRotator (Pawn|GetControlRotation :!class /Script/Engine.Pawn))))) AxisValue false))

(event Input|AxisEvents|InputAxisMoveRight
  (params (AxisValue :type Float%20%28single-precision%29))
  ;[0 1 0.1055] Basic Movement
  (Pawn|Input|AddMovementInput (Math|Vector|GetRightVector (Math|Rotator|MakeRotator 0.0 0.0 (.Yaw (Math|Rotator|BreakRotator (Pawn|GetControlRotation :!class /Script/Engine.Pawn))))) AxisValue false))

(fn ConstructionScript)

(fn SkillGDDShield
  (params (Destroy%20on%20hit? :type Boolean))
  (Variables|Default|SethasShield true)
  (Variables|Default|SetshieldDestroyOnHit Destroy%20on%20hit?)
  (Components|StaticMesh|SetStaticMesh (Variables|Default|GetShield) "/Game/Meshes/EditorPH/1M_Cube.1M_Cube"))

(fn SkillPaintbrushHeal
  (CallFunction|HealPlayer 2.0))

(fn SkillProgramHack
  (bind _asdcu_game_state (Utilities|Casting|CastToDCU_GameState (Game|GetGameState)))
  (Variables|/Game/Behaviour/DCU_GameState.DCU_GameState_C|SetHackIsOn _asdcu_game_state true))

(fn CardFail)