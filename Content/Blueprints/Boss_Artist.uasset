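; Artist boss enemy that fights the player and ends the game through DCU_GameMode when its health runs out.
; Tick aims the Shooter at the player, and seeing the player fires palette projectiles on a cooldown.
; A rain big attack spawns at BeginPlay and once at the first and third health thresholds, while the middle one only sets its flag.
; Capsule overlaps with six player weapon classes subtract damage and play a sound.
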(event OnSeePawn(PawnSensing)
  (params (Pawn :type Pawn%20Object%20Reference))
  (Utilities|Casting|CastToSkilledCharacter Pawn)
  (Utilities|FlowControl|Sequence
    (:then_0
      (if (<= (Variables|Default|GetBasic_Health) 7.5e+02)
        (if (Variables|Default|GetfirstTimeCompleted)
          (if (<= (Variables|Default|GetBasic_Health) 5e+02)
            (if (Variables|Default|GetsecondTimeCompleted)
              (if (<= (Variables|Default|GetBasic_Health) 2.5e+02)
                (if (not (Variables|Default|GetthirdTimeCompleted))
                  (Variables|Default|SetthirdTimeCompleted true)
                  (CallFunction|BigAttack)))
              (else
                (Variables|Default|SetsecondTimeCompleted true))))
          (else
            (Variables|Default|SetfirstTimeCompleted true)
            (CallFunction|BigAttack)))))
    (:then_1
      (if (Variables|Default|GetcanShoot)
        (CallFunction|Shoot)))))

(event OnComponentBeginOverlap(CapsuleComponent)
  (params (OverlappedComponent :type Primitive%20Component%20Object%20Reference) (OtherActor :type Actor%20Object%20Reference) (OtherComp :type Primitive%20Component%20Object%20Reference) (OtherBodyIndex :type Integer) (bFromSweep :type Boolean) (SweepResult :type Hit%20Result%20Structure%20%28by%20ref%29))
  (bind _asweapon_art (Utilities|Casting|CastToWeapon_Art OtherActor)
    (:then
      (CallFunction|BasicDamaged (Variables|/Game/Blueprints/Weapon_Art.Weapon_Art_C|GetDamage _asweapon_art)))
    (:CastFailed
      (bind _asweapon_design (Utilities|Casting|CastToWeapon_Design OtherActor)
        (:then
          (CallFunction|BasicDamaged (Variables|/Game/Blueprints/Weapon_Design.Weapon_Design_C|GetDamage _asweapon_design)))
        (:CastFailed
          (bind _asweapon_dev (Utilities|Casting|CastToWeapon_Dev OtherActor)
            (:then
              (CallFunction|BasicDamaged (Variables|/Game/Blueprints/Weapon_Dev.Weapon_Dev_C|GetDamage _asweapon_dev)))
            (:CastFailed
              (bind _asweapon_art_supper (Utilities|Casting|CastToWeapon_ArtSupper OtherActor)
                (:then
                  (CallFunction|BasicDamaged (Variables|/Game/Blueprints/Weapon_ArtSupper.Weapon_ArtSupper_C|GetDamage _asweapon_art_supper)))
                (:CastFailed
                  (bind _asweapon_design_supper (Utilities|Casting|CastToWeapon_DesignSupper OtherActor)
                    (:then
                      (CallFunction|BasicDamaged (Variables|/Game/Blueprints/Weapon_DesignSupper.Weapon_DesignSupper_C|GetDamage _asweapon_design_supper)))
                    (:CastFailed
                      (bind _asweapon_dev_super (Utilities|Casting|CastToWeapon_DevSuper OtherActor))
                      (CallFunction|BasicDamaged (Variables|/Game/Blueprints/Weapon_DevSuper.Weapon_DevSuper_C|GetDamage _asweapon_dev_super))))))))))))
  (Audio|PlaySound2D 0 1.0 1.0 0.0 0 0))

(event Custom|BasicDamaged
  (params (Damage :type Float%20%28single-precision%29))
  (Variables|Default|SetBasic_Health (- (Variables|Default|GetBasic_Health) Damage)))

(event Custom|Shoot
  (if (Variables|Default|GetcanShoot)
    (Variables|Default|SetcanShoot false)
    (Game|SpawnActorfromClass "/Game/Blueprints/EnemyWeapon_Palette.EnemyWeapon_Palette_C" (Transformation|GetWorldTransform (Variables|Default|GetShooter)) "Undefined" 0 0)
    (Utilities|FlowControl|Delay (Variables|Default|GetshootDelay))
    (Variables|Default|SetcanShoot true)))

(event Custom|BigAttack
  (Game|SpawnActorfromClass "/Game/Blueprints/EnemyWeapon_Boss_Rain1.EnemyWeapon_Boss_Rain1_C" (Transformation|GetWorldTransform (Variables|Default|GetBigAttack_Centre)) "Undefined" 0 0))

(event EventBeginPlay
  (CallFunction|BigAttack))

(event EventTick
  (params (DeltaSeconds :type Float%20%28single-precision%29))
  (Utilities|FlowControl|Sequence
    (:then_0
      (if (<= (Variables|Default|GetBasic_Health) 0.0)
        (bind _asdcu_game_mode (Utilities|Casting|CastToDCU_GameMode (Game|GetGameMode)))
        (Default|FinishedGame _asdcu_game_mode)
        (Actor|DestroyActor)
        (else
          (bind _asskilled_character (Utilities|Casting|CastToSkilledCharacter (Game|Player|GetPlayerPawn 0)))
          (Transformation|SetWorldRotation (Variables|Default|GetShooter) (Math|Rotator|FindLookatRotation (Transformation|GetWorldLocation (Variables|Default|GetShooter)) (Transformation|GetWorldLocation (Variables|/Script/Engine.Character|GetCapsuleComponent _asskilled_character))) false false))))))

(fn ConstructionScript)