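; Player character for a card-based ability game, with camera-yaw-relative movement, a cooldown-gated dash and health capped on Tick.
; Players cycle six single-use cards: three attacks and three skills (shield flag, timed paintbrush heal, program hack).
; Reload re-enables every card after a delay that grows with each use.
; Attack functions and CardFail are empty stubs, and the hack only casts to DCU_GameState.
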(event Custom|Reload
  (params (Duration :type Float%20%28single-precision%29))
  ;[0.07827 0 1] Reload Cards
  (Development|PrintString "Reload")
  (Utilities|FlowControl|Delay Duration)
  (Variables|Default|SetCard0_Disabled false)
  (Variables|Default|SetCard1_Disabled false)
  (Variables|Default|SetCard2_Disabled false)
  (Variables|Default|SetCard3_Disabled false)
  (Variables|Default|SetCard4_Disabled false)
  (Variables|Default|SetCard5_Disabled false)
  (Variables|Default|SetcanReload true))

(event Custom|DamagePlayer
  (params (Damage :type Float%20%28single-precision%29))
  ;[1 0.02997 0] Health Functions
  (Variables|Default|SetHealth (- (Variables|Default|GetHealth) Damage)))

(event Custom|HealPlayer
  (params (Healing :type Float%20%28single-precision%29))
  ;[1 0.02997 0] Health Functions
  (Variables|Default|SetHealth (+ (Variables|Default|GetHealth) Healing)))

(event EventTick
  (params (DeltaSeconds :type Float%20%28single-precision%29))
  (Utilities|FlowControl|Sequence
    (:then_0
      ;[1 1 1] Fixing Overhealth
      (if (> (Variables|Default|GetHealth) 1e+02)
        (Variables|Default|SetHealth 1e+02)))))

(event Input|ActionEvents|InputActionNextCard
  (params (Key :type Key%20Structure :default "None"))
  ;[0.973 0.2339 1] Next/Previous Card
  (:Pressed
    (if (>= (Variables|Default|GetCurrentCard) 5)
      (Variables|Default|SetCurrentCard 0)
      (else
        (Math|Integer|IncrementInt (Variables|Default|GetCurrentCard))))))

(event Input|ActionEvents|InputActionPrevCard
  (params (Key :type Key%20Structure :default "None"))
  ;[0.973 0.2339 1] Next/Previous Card
  (:Pressed
    (if (<= (Variables|Default|GetCurrentCard) 0)
      (Variables|Default|SetCurrentCard 5)
      (else
        (Math|Integer|DecrementInt (Variables|Default|GetCurrentCard))))))

(event Input|ActionEvents|InputActionDash
  (params (Key :type Key%20Structure :default "None"))
  ;[1 0.8526 0] Dash Ability
  (:Pressed
    (if (Variables|Default|GetcanDash)
      (Character|LaunchCharacter (* (Math|Vector|GetForwardVector (Variables|MyCharacter|GetCameraBoom)) 1e+04) false false)
      (Variables|Default|SetcanDash false)
      (Utilities|FlowControl|Delay 1.0)
      (Variables|Default|SetcanDash true))))

(event Input|ActionEvents|InputActionUseCard
  (params (Key :type Key%20Structure :default "None"))
  ;[0 0.9379 1] Using Cards
  (:Pressed
    (switch int (Variables|Default|GetCurrentCard)
      (:0
        (if (Variables|Default|GetCard0_Disabled)
          (CallFunction|CardFail)
          (else
            (Variables|Default|SetCard0_Disabled true)
            (CallFunction|AttackArt))))
      (:1
        (if (Variables|Default|GetCard1_Disabled)
          (CallFunction|CardFail)
          (else
            (Variables|Default|SetCard1_Disabled true)
            (CallFunction|AttackDesign))))
      (:2
        (if (Variables|Default|GetCard2_Disabled)
          (CallFunction|CardFail)
          (else
            (Variables|Default|SetCard2_Disabled true)
            (CallFunction|AttackDev))))
      (:3
        (if (Variables|Default|GetCard3_Disabled)
          (CallFunction|CardFail)
          (else
            (Variables|Default|SetCard3_Disabled true)
            (CallFunction|SkillGDDShield))))
      (:4
        (if (Variables|Default|GetCard4_Disabled)
          (CallFunction|CardFail)
          (else
            (Variables|Default|SetCard4_Disabled true)
            (bind _returnvalue (Utilities|Time|SetTimerbyFunctionName 0 "Skill_PaintbrushHeal" 0.2 true))
            (Utilities|FlowControl|Delay 1.0)
            (Utilities|Time|ClearandInvalidateTimerbyHandle _returnvalue))))
      (:5
        (if (Variables|Default|GetCard5_Disabled)
          (CallFunction|CardFail)
          (else
            (Variables|Default|SetCard5_Disabled true)
            (CallFunction|SkillProgramHack)))))))

(event Input|ActionEvents|InputActionReload
  (params (Key :type Key%20Structure :default "None"))
  (bind _reloadtime (Variables|Default|GetReloadTime))
  ;[0.973 0.2339 1] Next/Previous Card
  (:Pressed
    (if (Variables|Default|GetcanReload)
      (Variables|Default|SetcanReload false)
      (CallFunction|Reload (Math|Conversions|ToFloat(Integer) _reloadtime))
      (Math|Integer|IncrementInt _reloadtime))))

(event Input|AxisEvents|InputAxisMoveForward
  (params (AxisValue :type Float%20%28single-precision%29))
  ;[0 1 0.1055] Basic Movement
  (Pawn|Input|AddMovementInput (Math|Vector|GetForwardVector (Math|Rotator|MakeRotator 0.0 0.0 (.Yaw (Math|Rotator|BreakRotator (Pawn|GetControlRotation :!class /Script/Engine.Pawn))))) AxisValue false))

(event Input|AxisEvents|InputAxisMoveRight
  (params (AxisValue :type Float%20%28single-precision%29))
  ;[0 1 0.1055] Basic Movement
  (Pawn|Input|AddMovementInput (Math|Vector|GetRightVector (Math|Rotator|MakeRotator 0.0 0.0 (.Yaw (Math|Rotator|BreakRotator (Pawn|GetControlRotation :!class /Script/Engine.Pawn))))) AxisValue false))

(fn ConstructionScript)

(fn AttackDesign)

(fn AttackDev)

(fn AttackArt)

(fn SkillGDDShield
  (Variables|Default|SethasShield true))

(fn SkillPaintbrushHeal
  (CallFunction|HealPlayer 2.0))

(fn SkillProgramHack
  (Utilities|Casting|CastToDCU_GameState (Game|GetGameState)))

(fn CardFail)